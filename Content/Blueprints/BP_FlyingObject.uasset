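; BP_FlyingObject is a moving target that awards score to the instigating player when damaged.
; Tick adds a time-based sine step on X to its current location, so motion is frame-rate dependent, with a randomized starting phase.
; AnyDamage increments the instigator's MyPlayerState score on authority only; the following MyGameMode cast leads nowhere.
; It expires through a fixed lifespan set at BeginPlay, not on damage.
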(event Collision|EventActorBeginOverlap
  (params (OtherActor :type Actor%20Object%20Reference)))

(event EventTick
  (params (DeltaSeconds :type Float%20%28single-precision%29))
  (bind _output_get (Variables|Default|SetTime%20count (+ DeltaSeconds (Variables|Default|GetTime%20count))))
  (Transformation|SetActorLocation self (+ (Transformation|GetActorLocation) (Math|Vector|MakeVector (* (Math|Trig|Sin(Radians) (Math|Float|MultiplybyPi (/ _output_get (Variables|Default|GetT)))) 6e+01) 0.0 0.0)) false false))

(event Game|Damage|EventAnyDamage
  (params (Damage :type Float%20%28single-precision%29) (DamageType :type Damage%20Type%20Object%20Reference) (InstigatedBy :type Controller%20Object%20Reference) (DamageCauser :type Actor%20Object%20Reference))
  (if (Utilities|IsValid InstigatedBy)
    (Networking|SwitchHasAuthority
      (:Authority
        (bind _asmy_player_state (Utilities|Casting|CastToMyPlayerState (Variables|/Script/Engine.Controller|GetPlayerState InstigatedBy))
          (:then
            (Default|IncrementScore _asmy_player_state))
          (:CastFailed
            _))
        (Utilities|Casting|CastToMyGameMode (Game|GetGameMode))))))

(event EventBeginPlay
  (Variables|Default|Setself%20loc (Transformation|GetActorLocation))
  (Variables|Default|SetTime%20count (Math|Random|RandomFloatinRange 0.0 (Variables|Default|GetT)))
  (Actor|SetLifeSpan 1.2e+02))

(fn ConstructionScript)